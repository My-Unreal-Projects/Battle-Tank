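; Mortar pawn or actor Blueprint that sets up a mortar emplacement with aiming, projectile firing setup, aiming audio and a health bar.
; BeginPlay hands the barrel, turret, projectile class and reload time to the MortarAiming component, which owns the aiming logic.
; Each Tick polls that component for barrel movement to raise or mute the aiming sound.
; The red-tinted health bar widget reuses HealthBar_BP, receiving the mortar through its Tank reference.
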(event `self.ReceiveBeginPlay`
  (`TankAimingComponent.Initialise` (`self.MortarAiming`) (`self.Barrel`) (`self.Turret`) "/Game/Projectile/Projectile_BP.Projectile_BP_C" 4.0)
  (`self.InitialiseHealthBarWidget`))

(event `self.ReceiveTick`
  (params (DeltaSeconds :type "Float (single-precision)"))
  (bind _mortaraimingaudio (`self.MortarAimingAudio`))
  ;[1 1 1] Aiming Audio Setup
  (bind _returnvalue (`TankAimingComponent.IsBarrelMoving` (`self.MortarAiming`)))
  (if _returnvalue
    (`AudioComponent.SetVolumeMultiplier` _mortaraimingaudio 0.1)
    (else
      (`AudioComponent.SetVolumeMultiplier` _mortaraimingaudio 0.0))))

(fn `InitialiseHealthBarWidget`
  (bind _ashealth_bar_bp (cast `/Game/UI/HealthBar_BP` (`WidgetComponent.GetUserWidgetObject` (`self.HealthBar`))))
  (set `/Game/UI/HealthBar_BP.Tank` self _ashealth_bar_bp)
  (`UserWidget.SetColorAndOpacity` _ashealth_bar_bp (struct :`R` 1.0 :`B` 0.027451 :`A` 1.0)))

(fn `UserConstructionScript`)