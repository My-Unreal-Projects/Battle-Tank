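; TankAIController_BP is the AI controller for enemy tanks that triggers the victory screen when the last one dies.
; On PossessedTankDead it counts the AI controllers of its class in the world and acts only if one or fewer remain.
; It then clears all widgets, shows EndMenuUI_BP with green VICTORY text and enables the mouse cursor.
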(event `self.PossessedTankDead`
  (bind _outactors (`GameplayStatics.GetAllActorsOfClass` "TankAIController_BP_C"))
  (if (<= (`KismetArrayLibrary.Array_Length` _outactors) 1)
    ;[1 1 1] Initialise Victory End Menu
    (`WidgetLayoutLibrary.RemoveAllWidgets`)
    (bind _returnvalue (`|CreateWidget` "/Game/UI/EndMenuUI_BP.EndMenuUI_BP_C"))
    (`UserWidget.AddToViewport` _returnvalue 0)
    (set `PlayerController.bShowMouseCursor` true (`GameplayStatics.GetPlayerController` 0))
    (set `/Game/UI/EndMenuUI_BP.ResultText` "VICTORY" _returnvalue)
    (set `/Game/UI/EndMenuUI_BP.TextColor` (make `SlateColor` (struct :`G` 1.0 :`B` 0.284322 :`A` 1.0)) _returnvalue)
    (`/Game/UI/EndMenuUI_BP.WidgetReady` _returnvalue)))

(fn `UserConstructionScript`)