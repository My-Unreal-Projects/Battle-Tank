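; Game mode for the battle tank game that shows the main menu on play and sets up the match when it starts.
; BeginPlay creates the menu widget with the mouse cursor visible.
; StartGame spawns the player tank, possesses it and blends the camera to it, then spawns an enemy tank and mortars at hard-coded locations.
; Some extra enemy spawns are left disconnected and never run.
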(event `self.ReceiveBeginPlay`
  ;[1 1 1] Main menu set up
  (bind _returnvalue (`|CreateWidget` "/Game/UI/MainMenuUI_BP.MainMenuUI_BP_C"))
  (`UserWidget.AddToViewport` _returnvalue 0)
  (set `PlayerController.bShowMouseCursor` true (`GameplayStatics.GetPlayerController` 0))
  (`/Game/UI/MainMenuUI_BP.WidgetReady` _returnvalue))

(event `Start Game`
  ;[1 1 1] Initialise Game
  (`self.InitPlayerTank`)
  (`self.InitEnemies`))

(fn `InitEnemies`
  (`|SpawnActorFromClass` "/Game/Tank/EnemyTank_BP.EnemyTank_BP_C" (`KismetMathLibrary.Conv_VectorToTransform` (-7160.0 -1100.0 70.0)) "AdjustIfPossibleButAlwaysSpawn" "OverrideRootScale" null null)
  (`|SpawnActorFromClass` "/Game/Mortar/Mortar_BP.Mortar_BP_C" (`KismetMathLibrary.Conv_VectorToTransform` (-10560.0 -1370.0 -140.0)) "AdjustIfPossibleButAlwaysSpawn" "OverrideRootScale" null null)
  (`|SpawnActorFromClass` "/Game/Mortar/Mortar_BP.Mortar_BP_C" (`KismetMathLibrary.Conv_VectorToTransform` (-4830.0 -8590.0 10.0)) "AdjustIfPossibleButAlwaysSpawn" "OverrideRootScale" null null)
  (`|SpawnActorFromClass` "/Game/Mortar/Mortar_BP.Mortar_BP_C" (`KismetMathLibrary.Conv_VectorToTransform` (-5030.0 7910.0 -20.0)) "AdjustIfPossibleButAlwaysSpawn" "OverrideRootScale" null null))

(fn `InitPlayerTank`
  (bind _returnvalue (`GameplayStatics.GetPlayerController` 0))
  (bind _returnvalue_2 (`|SpawnActorFromClass` "/Game/Tank/Tank_BP.Tank_BP_C" (`KismetMathLibrary.Conv_VectorToTransform` (8070.0 -5120.0 -150.0)) "AdjustIfPossibleButAlwaysSpawn" "OverrideRootScale" null null))
  (`Controller.Possess` _returnvalue _returnvalue_2)
  (bind _astank_player_controller_bp (cast `/Game/Blueprints/TankPlayerController_BP` _returnvalue))
  (`PlayerController.SetViewTargetWithBlend` _astank_player_controller_bp _returnvalue_2 1.5 "VTBlend_Linear" 0.0 false))

(fn `UserConstructionScript`)